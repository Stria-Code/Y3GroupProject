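; Sliding door Blueprint that opens for a first-person character with sufficient clearance.
; Entering the trigger box compares the character's AccessLevel against DoorClearance and, if high enough, plays the DoorMovement timeline.
; The timeline's DoorOpen track lerps the door mesh's relative Z location from zero to OpenValue.
; Leaving the box reverses the timeline for any first-person character, without rechecking clearance.
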(event `self.Box.OnComponentBeginOverlap`
  (params (OverlappedComponent :type "PrimitiveComponent Object Reference") (OtherActor :type "Actor Object Reference") (OtherComp :type "PrimitiveComponent Object Reference") (OtherBodyIndex :type Integer) (bFromSweep :type Boolean) (SweepResult :type "HitResult Structure (by ref)"))
  (bind _asbp_first_person_character (cast `/Game/FirstPerson/Blueprints/BP_FirstPersonCharacter` OtherActor))
  (if (>= (`GroupProjectY3Character.accessLevel` _asbp_first_person_character) (`self.DoorClearance`))
    (bind (_direction _dooropen) (`Timeline|DoorMovement` :!label _label)
      (:`Update`
        (`SceneComponent.K2_SetRelativeLocation` (`self.Door`) (`KismetMathLibrary.MakeVector` 0.0 0.0 (`KismetMathLibrary.Lerp` 0.0 (`self.OpenValue`) _dooropen)) false false)))))

(event `self.Box.OnComponentEndOverlap`
  (params (OverlappedComponent :type "PrimitiveComponent Object Reference") (OtherActor :type "Actor Object Reference") (OtherComp :type "PrimitiveComponent Object Reference") (OtherBodyIndex :type Integer))
  (cast `/Game/FirstPerson/Blueprints/BP_FirstPersonCharacter` OtherActor)
  (goto _label :!via `Reverse`))

(fn `UserConstructionScript`)