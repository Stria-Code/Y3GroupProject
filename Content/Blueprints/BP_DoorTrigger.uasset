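; Door trigger actor that activates every SlidingDoor tagged with its TargetTag when any actor overlaps it.
; For each door, if DestroyTriggers is valid, it also destroys DialogueInator actors sharing that tag.
; It then destroys itself, though with DestroyTriggers valid this happens only inside the DialogueInator loop, so it persists when none are found.
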(event `self.ReceiveActorBeginOverlap`
  (params (OtherActor :type "Actor Object Reference"))
  (bind _outactors (`GameplayStatics.GetAllActorsOfClassWithTag` "/Game/Blueprints/SlidingDoor.SlidingDoor_C" (`KismetStringLibrary.Conv_StringToName` (`self.TargetTag`))))
  (for _array_element _outactors
    (set `/Game/Blueprints/SlidingDoor.DoorActive` true _array_element)
    (`self.DestroyTriggers`
      (:`then`
        (bind _outactors_2 (`GameplayStatics.GetAllActorsOfClassWithTag` "/Game/Blueprints/Dialogue/DialogueInator.DialogueInator_C" (`KismetStringLibrary.Conv_StringToName` (`self.TargetTag`))))
        (for _array_element_2 _outactors_2
          (`self.K2_DestroyActor` _array_element_2)
          (`self.K2_DestroyActor` :!label _label)))
      (:`else`
        (goto _label)))))

(fn `UserConstructionScript`)