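; Interactable note actor that the player can pick up to inspect and then return to its original place.
; Interact alternates via a FlipFlop: first, a timeline lerps the note to the character's INotePoint while movement and look are locked, the cursor shows and camera blur turns on.
; The next interaction snaps it back, restores controls and resumes the Chronovert timer paused on interaction.
; Look-target events toggle its prompt widget.
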(event `self.ReceiveBeginPlay`
  (bind _object (`self.Object`))
  (set `self.Original Loc` (`SceneComponent.K2_GetComponentLocation` _object))
  (set `self.Original Rot` (`SceneComponent.K2_GetComponentRotation` _object))
  (`self.EnableInput` (`GameplayStatics.GetPlayerController` 0)))

(event `InteractableInterface.Interact`
  (params (InteractingActor :type "Actor Object Reference"))
  (bind _returnvalue (`GameplayStatics.GetPlayerController` 0))
  (bind _object (`self.Object`))
  (bind _widget (`self.Widget`))
  (`InteractableInterface.InteractPauseChronovertTimer`)
  (if (`self.CanInteract`)
    (`/Engine/EditorBlueprintResources/StandardMacros.FlipFlop`
      (:`A`
        (`SceneComponent.SetVisibility` _widget false false)
        (`/Engine/EditorBlueprintResources/StandardMacros.DoOnce` false :!label _label
          (:`Completed`
            (set `self.CanInteract` false)
            (`CharacterMovementComponent.DisableMovement` (`Character.CharacterMovement` (`GameplayStatics.GetPlayerCharacter` 0)))
            (set `self.CanShowWidget` false)
            (set `PlayerController.bShowMouseCursor` true (`GameplayStatics.GetPlayerController` 0))
            (set `self.CanInspect` true)
            (`GameplayStatics.PlaySound2D` "/Game/Sound/PaperFlutterSFX.PaperFlutterSFX" 1.0 1.0 0.0 null null)
            (bind _asbp_first_person_character (cast `/Game/FirstPerson/Blueprints/BP_FirstPersonCharacter` (`GameplayStatics.GetPlayerCharacter` 0)))
            (`/Game/FirstPerson/Blueprints/BP_FirstPersonCharacter.SetInspectCamBlur` _asbp_first_person_character true 30.0)
            (`Controller.SetIgnoreLookInput` (`GameplayStatics.GetPlayerController` 0) true)
            (bind (_direction _newtrack_0) (`Timeline|Timeline` :!via `PlayFromStart`)
              (:`Update`
                (bind (_returnvalue_location _returnvalue_rotation) (`KismetMathLibrary.BreakTransform` (`SceneComponent.K2_GetComponentToWorld` (`/Game/FirstPerson/Blueprints/BP_FirstPersonCharacter.INotePoint` _asbp_first_person_character))))
                (`SceneComponent.K2_SetWorldTransform` (`self.Object`) (`KismetMathLibrary.MakeTransform` (`KismetMathLibrary.VLerp` (`SceneComponent.K2_GetComponentLocation` _object) _returnvalue_location _newtrack_0) (`KismetMathLibrary.RLerp` (`SceneComponent.K2_GetComponentRotation` _object) _returnvalue_rotation _newtrack_0)) false false))
              (:`Finished`
                (set `self.CanInteract` true))))))
      (:`B`
        (`SceneComponent.SetVisibility` _widget true false)
        (`|ExecutionSequence`
          (:`then_0`
            (goto _label :!via `Reset`))
          (:`then_1`
            (`SceneComponent.K2_SetWorldTransform` (`self.Object`) (`KismetMathLibrary.MakeTransform` (`self.Original Loc`) (`self.Original Rot`)) false false)
            (set `self.CanInspect` false)
            (set `self.CanShowWidget` true)
            (`CharacterMovementComponent.SetMovementMode` (`Character.CharacterMovement` (`GameplayStatics.GetPlayerCharacter` 0)) "MOVE_Walking" 0)
            (set `PlayerController.bShowMouseCursor` false _returnvalue)
            (`Controller.ResetIgnoreLookInput` _returnvalue)
            (`WidgetBlueprintLibrary.SetInputMode_GameOnly` _returnvalue)
            (set `self.CanInteract` true)
            (bind _asbp_first_person_character_2 (cast `/Game/FirstPerson/Blueprints/BP_FirstPersonCharacter` (`GameplayStatics.GetPlayerCharacter` 0)))
            (`/Game/FirstPerson/Blueprints/BP_FirstPersonCharacter.SetInspectCamBlur` _asbp_first_person_character_2 false 0.0)
            (`InteractableInterface.InteractResumeChronovertTimer`)))))))

(event `InteractableInterface.LookTargetEvent`
  (params (isLooking :type Boolean))
  (bind _widget (`self.Widget`))
  ; Enable/Disable Widget
  (`self.CanShowWidget`
    (:`then`
      (if isLooking
        (`SceneComponent.SetVisibility` _widget true false)
        (else
          (`SceneComponent.SetVisibility` _widget false false))))
    (:`else`)))

(fn `UserConstructionScript`)