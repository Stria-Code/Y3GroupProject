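; Ceiling light Blueprint with a spot light and a bounce light that can be switched through a SetTechActive event.
; BeginPlay sets both lights' visibility from IsOnAtStart, and SetTechActive sets it from IsActive.
; Both events also swap material slot 1 on static mesh children of Lights, but BeginPlay always applies OffMat and SetTechActive always applies OnMat, whatever the on/off state.
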(event `self.ReceiveBeginPlay`
  (bind _isonatstart (`self.IsOnAtStart`))
  (`SceneComponent.SetVisibility` (`self.SpotLight`) _isonatstart false)
  (`SceneComponent.SetVisibility` (`self.BounceLight`) _isonatstart false)
  (for _array_element (`SceneComponent.GetChildrenComponents` (`self.Lights`) false)
    (bind _asstatic_mesh_component (cast `StaticMeshComponent` _array_element))
    (`PrimitiveComponent.SetMaterial` _asstatic_mesh_component 1 (`self.OffMat`))))

(event `/Game/Blueprints/Interface/BPI_Tech.SetTechActive`
  (params (IsActive :type Boolean))
  (`SceneComponent.SetVisibility` (`self.SpotLight`) IsActive false)
  (`SceneComponent.SetVisibility` (`self.BounceLight`) IsActive false)
  (for _array_element (`SceneComponent.GetChildrenComponents` (`self.Lights`) false)
    (bind _asstatic_mesh_component (cast `StaticMeshComponent` _array_element))
    (`PrimitiveComponent.SetMaterial` _asstatic_mesh_component 1 (`self.OnMat`))))

(fn `UserConstructionScript`)