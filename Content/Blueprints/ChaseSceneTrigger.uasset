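; Trigger actor for the chase sequence that acts only when the player overlaps it after downloading the data.
; If its IsChaseEnd reference is valid, it opens the OutroSequence level once through a DoOnce.
; Otherwise it plays an alarm sound and turns point lights carrying the target tag red, with no guard against repeat overlaps.
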(event `self.ReceiveActorBeginOverlap`
  (params (OtherActor :type "Actor Object Reference"))
  (bind _returnvalue (`GameplayStatics.GetPlayerCharacter` 0))
  (bind _asbp_first_person_character (cast `/Game/FirstPerson/Blueprints/BP_FirstPersonCharacter` _returnvalue))
  (if (and (== OtherActor _returnvalue) (`GroupProjectY3Character.hasDownloadedData` _asbp_first_person_character))
    (`self.IsChaseEnd`
      (:`then`
        (`/Engine/EditorBlueprintResources/StandardMacros.DoOnce` false
          (:`Completed`
            (`GameplayStatics.OpenLevel` "OutroSequence"))))
      (:`else`
        (`GameplayStatics.PlaySound2D` "/Game/Sound/AlarmSFX.AlarmSFX" 1.0 1.0 0.0 null null)
        (bind _outactors (`GameplayStatics.GetAllActorsOfClassWithTag` "/Script/Engine.PointLight" (`self.TargetTag`)))
        (for _array_element _outactors
          (`LightComponent.SetLightColor` (`Light.LightComponent` _array_element) (struct :`R` 1.0 :`G` 0.043051 :`A` 1.0) true))))))

(fn `UserConstructionScript`)