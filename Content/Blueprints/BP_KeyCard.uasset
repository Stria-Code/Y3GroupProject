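; BP_KeyCard is an interactable key card actor that shows a widget while looked at and plays subtitle dialogue on interaction.
; The widget starts hidden and follows the look-target event's state.
; Interaction prints a debug greeting, then, if DialogueTable is valid, a DoOnce clears existing W_Subtitles and creates a new one from row "1".
; No pickup or unlock logic is present.
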(event `self.ReceiveBeginPlay`
  (`SceneComponent.SetVisibility` (`self.Widget`) false false))

(event `InteractableInterface.LookTargetEvent`
  (params (isLooking :type Boolean))
  (`SceneComponent.SetVisibility` (`self.Widget`) isLooking false))

(event `InteractableInterface.InteractionDialogue`
  (params (InteractingActor :type "Actor Object Reference"))
  (`KismetSystemLibrary.PrintString` "Hello")
  (bind _dialoguetable (`self.DialogueTable`)
    (:`then`
      (`/Engine/EditorBlueprintResources/StandardMacros.DoOnce` false
        (:`Completed`
          (bind _foundwidgets (`WidgetBlueprintLibrary.GetAllWidgetsOfClass` "/Game/Dialogue/W_Subtitles.W_Subtitles_C"))
          (for _array_element _foundwidgets
            (`/Game/Dialogue/W_Subtitles.RemoveDialogue` _array_element))
          (bind _returnvalue (`|CreateWidget` "/Game/Dialogue/W_Subtitles.W_Subtitles_C" null (make `DataTableRowHandle` _dialoguetable "1")))
          (`UserWidget.AddToViewport` _returnvalue 0))))
    (:`else`)))

(fn `UserConstructionScript`)