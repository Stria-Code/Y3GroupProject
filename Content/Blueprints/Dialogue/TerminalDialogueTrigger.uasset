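; One-shot trigger actor that updates dialogue on tagged door terminals when the player character overlaps it.
; It finds every BP_DoorTerminal with TargetTag and applies SetEnabled to its dialogue.
; It also assigns NewTable when an IsValid check passes, though that check reads SetEnabled rather than the table.
; The trigger destroys itself afterward.
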(event `self.ReceiveActorBeginOverlap`
  (params (OtherActor :type "Actor Object Reference"))
  (if (== OtherActor (`GameplayStatics.GetPlayerCharacter` 0))
    (bind _outactors (`GameplayStatics.GetAllActorsOfClassWithTag` "/Game/Blueprints/BP_DoorTerminal.BP_DoorTerminal_C" (`self.TargetTag`)))
    (for _array_element _outactors
      (bind _setenabled (`self.SetEnabled`)
        (:`then`
          (`/Game/Blueprints/BP_DoorTerminal.SetDialogueTable` _array_element (`self.New Table`))
          (`/Game/Blueprints/BP_DoorTerminal.SetDialogueEnabled` _array_element _setenabled))
        (:`else`
          (`/Game/Blueprints/BP_DoorTerminal.SetDialogueEnabled` _array_element _setenabled))))
    (`self.K2_DestroyActor`)))

(fn `UserConstructionScript`)