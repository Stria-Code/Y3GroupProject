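; DialogueInator is a trigger actor that shows subtitle dialogue when the player overlaps it.
; On overlap, a DoOnce, optionally starting disabled, clears existing W_Subtitles widgets, creates a new one from row "1" of DialogueTable and can destroy the trigger.
; External events re-enable it, firing immediately if the player is inside, or destroy it.
; StartDisplaced offsets it far along Y at BeginPlay until UnDisplace moves it back.
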(event `UnDisplace`
  (`self.K2_AddActorWorldOffset` (0.0 6000.0 0.0)))

(event `self.ReceiveBeginPlay`
  (`self.StartDisplaced`
    (:`then`
      (`self.K2_AddActorWorldOffset` (0.0 -6000.0 0.0)))
    (:`else`)))

(event `self.ReceiveActorBeginOverlap`
  (params (OtherActor :type "Actor Object Reference"))
  (if (== OtherActor (`GameplayStatics.GetPlayerCharacter` 0))
    (`/Engine/EditorBlueprintResources/StandardMacros.DoOnce` (`self.StartDisabled`) :!label _label
      (:`Completed`
        (bind _foundwidgets (`WidgetBlueprintLibrary.GetAllWidgetsOfClass` "/Game/Dialogue/W_Subtitles.W_Subtitles_C"))
        (for _array_element _foundwidgets
          (`/Game/Dialogue/W_Subtitles.RemoveDialogue` _array_element))
        (bind _returnvalue (`|CreateWidget` "/Game/Dialogue/W_Subtitles.W_Subtitles_C" null (make `DataTableRowHandle` (`self.DialogueTable`) "1")))
        (`UserWidget.AddToViewport` _returnvalue 0)
        (if (`self.DeleteAfterPlay`)
          (`self.K2_DestroyActor` :!label _label_2))))))

(event `DestroyTrigger`
  (goto _label_2))

(event `ReEnableDialogue`
  (`|ExecutionSequence`
    (:`then_0`
      (goto _label :!via `Reset`))
    (:`then_1`
      (if (`self.IsOverlappingActor` (`GameplayStatics.GetPlayerCharacter` 0))
        (goto _label)))))

(fn `UserConstructionScript`)