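; An interactable in-world computer that moves the first-person camera to its screen and hosts the P3 puzzle widget.
; Interact toggles entry and exit via FlipFlop, using timelines to blend the camera and scale the screen while switching input, movement and chronovert timer pause.
; The widget receives a reference to the computer.
; Start, exit and download events re-enable tagged DialogueInators; code upload releases the player and reveals tagged keycards.
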(event `self.ReceiveBeginPlay`
  (`SceneComponent.SetVisibility` (`self.InteractWidget`) false false)
  (`SceneComponent.SetVisibility` (`self.ScreenWidget`) false false)
  (bind _ascomp_p3pass (cast `/Game/UI/BlueprintUI/Comp_P3Pass` (`WidgetComponent.GetUserWidgetObject` (`self.ScreenWidget`))))
  (bind _comp_p3 (`/Game/UI/BlueprintUI/Comp_P3Pass.Comp_P3` _ascomp_p3pass))
  (set `/Game/UI/BlueprintUI/Comp_P3.Computer` self _comp_p3)
  (set `self.P3Widget` _comp_p3))

(event `InteractableInterface.LookTargetEvent`
  (params (isLooking :type Boolean))
  (bind _interactwidget (`self.InteractWidget`))
  (bind _canshowwidget (`self.CanShowWidget`)
    (:`then`
      (if true
        (`SceneComponent.SetVisibility` _interactwidget isLooking false)))
    (:`else`
      (`SceneComponent.SetVisibility` _interactwidget _canshowwidget false))))

(event `InteractableInterface.Interact`
  (params (InteractingActor :type "Actor Object Reference"))
  (bind _returnvalue (`GameplayStatics.GetPlayerController` 0))
  (bind _returnvalue_2 (`GameplayStatics.GetPlayerController` 0))
  (bind _interactwidget (`self.InteractWidget`))
  (bind (_playercamerapos_location _playercamerapos_rotation) (`KismetMathLibrary.BreakTransform` (`self.PlayerCameraPos`)))
  (bind _screenwidget (`self.ScreenWidget`))
  (bind (_returnvalue_location _returnvalue_rotation) (`KismetMathLibrary.BreakTransform` (`SceneComponent.K2_GetComponentToWorld` (`self.CameraPosition`))))
  (`|ExecutionSequence`
    (:`then_0`
      (`/Engine/EditorBlueprintResources/StandardMacros.DoOnce` false
        (:`Completed`
          (bind _outactors (`GameplayStatics.GetAllActorsOfClassWithTag` "/Game/Blueprints/Dialogue/DialogueInator.DialogueInator_C" (`self.StartDialogueTag`)))
          (for _array_element _outactors
            (bind _asdialogue_inator (cast `/Game/Blueprints/Dialogue/DialogueInator` _array_element))
            (`/Game/Blueprints/Dialogue/DialogueInator.ReEnableDialogue` _asdialogue_inator)
            (bind _p3widget (`self.P3Widget`)
              (:`then`
                (set `/Game/UI/BlueprintUI/Comp_P3.IsOnComputer` true _p3widget))
              (:`else`))))))
    (:`then_1`
      (message `InteractableInterface.InteractPauseChronovertTimer` self)
      (if (`self.CanInteract`)
        (`/Engine/EditorBlueprintResources/StandardMacros.FlipFlop`
          (:`A`
            (`SceneComponent.SetVisibility` _interactwidget false false)
            (`/Engine/EditorBlueprintResources/StandardMacros.DoOnce` false :!label _label
              (:`Completed`
                (bind _asbp_first_person_character (cast `/Game/FirstPerson/Blueprints/BP_FirstPersonCharacter` InteractingActor))
                (set `PlayerController.bShowMouseCursor` true _returnvalue)
                (`CharacterMovementComponent.DisableMovement` (`Character.CharacterMovement` _asbp_first_person_character))
                (`Controller.SetIgnoreLookInput` _returnvalue true)
                (bind _firstpersoncameracomponent (`GroupProjectY3Character.FirstPersonCameraComponent` _asbp_first_person_character))
                (set `self.PlayerCameraPos` (`SceneComponent.K2_GetComponentToWorld` _firstpersoncameracomponent))
                (set `self.CanInteract` false)
                (`WidgetBlueprintLibrary.SetInputMode_GameAndUIEx` _returnvalue (`WidgetComponent.GetUserWidgetObject` (`self.ScreenWidget`)))
                (`SceneComponent.SetWorldScale3D` _screenwidget (1.0 0.023 0.0))
                (`SceneComponent.SetVisibility` _screenwidget true false)
                (bind (_direction _movement) (`Timeline|CamMove` :!via `PlayFromStart` :!label _label_2)
                  (:`Update`
                    (bind _returnvalue_3 (`KismetMathLibrary.RLerp` _playercamerapos_rotation _returnvalue_rotation _movement))
                    (`SceneComponent.K2_SetWorldTransform` _firstpersoncameracomponent (`KismetMathLibrary.MakeTransform` (`KismetMathLibrary.VLerp` _playercamerapos_location _returnvalue_location _movement) _returnvalue_3) false false)
                    (`Controller.SetControlRotation` (`GameplayStatics.GetPlayerController` 0) _returnvalue_3))
                  (:`Finished`
                    (set `self.CanInteract` true)
                    (if (`self.IsExiting`)
                      (set `self.IsExiting` false)
                      (`CharacterMovementComponent.SetMovementMode` (`Character.CharacterMovement` (`GameplayStatics.GetPlayerCharacter` 0)) "MOVE_Walking" 0)
                      (set `PlayerController.bShowMouseCursor` false _returnvalue_2)
                      (`Controller.ResetIgnoreLookInput` _returnvalue_2)
                      (`WidgetBlueprintLibrary.SetInputMode_GameOnly` _returnvalue_2)
                      (set `self.CanInteract` true)
                      (message `InteractableInterface.InteractResumeChronovertTimer` self)
                      (bind _asbp_first_person_character_2 (cast `/Game/FirstPerson/Blueprints/BP_FirstPersonCharacter` (`GameplayStatics.GetPlayerCharacter` 0)))
                      (`GroupProjectY3Character.SetInspectingState` _asbp_first_person_character_2)
                      (`|ExecutionSequence`
                        (:`then_0`
                          (bind _p3widget_2 (`self.P3Widget`)
                            (:`then`
                              (set `/Game/UI/BlueprintUI/Comp_P3.IsOnComputer` false _p3widget_2)
                              (`/Engine/EditorBlueprintResources/StandardMacros.DoOnce` false
                                (:`Completed`
                                  (bind _outactors_2 (`GameplayStatics.GetAllActorsOfClassWithTag` "/Game/Blueprints/Dialogue/DialogueInator.DialogueInator_C" (`self.EndDialogueTag`)))
                                  (for _array_element_2 _outactors_2
                                    (bind _asdialogue_inator_2 (cast `/Game/Blueprints/Dialogue/DialogueInator` _array_element_2))
                                    (`/Game/Blueprints/Dialogue/DialogueInator.ReEnableDialogue` _asdialogue_inator_2)))))
                            (:`else`)))
                        (:`then_1`
                          (bind (_direction_2 _movement_2) (`Timeline|Timeline` :!via `ReverseFromEnd` :!label _label_3)
                            (:`Update`
                              (`SceneComponent.SetWorldScale3D` (`self.ScreenWidget`) (`KismetMathLibrary.MakeVector` 1.0 0.023 (`KismetMathLibrary.Lerp` 0.0 0.023 _movement_2))))
                            (:`Finished`
                              (if (`self.IsExiting`)
                                (`SceneComponent.SetVisibility` (`self.ScreenWidget`) false false))))))
                      (else
                        (`GameplayStatics.PlaySound2D` "/Game/Sound/ComputerTurnOnAlt.ComputerTurnOnAlt" 1.0 1.0 0.0 null null)
                        (goto _label_3 :!via `PlayFromStart`))))))))
          (:`B`
            (`SceneComponent.SetVisibility` _interactwidget true false)
            (`|ExecutionSequence`
              (:`then_0`
                (goto _label :!via `Reset`))
              (:`then_1`
                (set `self.CanInteract` false)
                (set `self.IsExiting` true)
                (goto _label_2 :!via `ReverseFromEnd`)))))))))

(event `CodeUpload`
  (bind _returnvalue (`GameplayStatics.GetPlayerController` 0))
  (`CharacterMovementComponent.SetMovementMode` (`Character.CharacterMovement` (`GameplayStatics.GetPlayerCharacter` 0)) "MOVE_Walking" 0)
  (set `PlayerController.bShowMouseCursor` false _returnvalue)
  (`Controller.ResetIgnoreLookInput` _returnvalue)
  (`WidgetBlueprintLibrary.SetInputMode_GameOnly` _returnvalue)
  (set `self.CanInteract` true)
  (message `InteractableInterface.InteractResumeChronovertTimer` self)
  (bind _asbp_first_person_character (cast `/Game/FirstPerson/Blueprints/BP_FirstPersonCharacter` (`GameplayStatics.GetPlayerCharacter` 0)))
  (`GroupProjectY3Character.SetInspectingState` _asbp_first_person_character)
  (bind _p3widget (`self.P3Widget`)
    (:`then`
      (set `/Game/UI/BlueprintUI/Comp_P3.IsOnComputer` false _p3widget)
      (bind _outactors (`GameplayStatics.GetAllActorsOfClassWithTag` "/Game/Blueprints/BP_KeyCard.BP_KeyCard_C" (`self.EndDialogueTag`)))
      (for _array_element _outactors
        (`self.SetActorHiddenInGame` _array_element false)))
    (:`else`)))

(event `DownloadBar`
  (`|ExecutionSequence`
    (:`then_0`
      (`/Engine/EditorBlueprintResources/StandardMacros.DoOnce` false
        (:`Completed`
          (bind _outactors (`GameplayStatics.GetAllActorsOfClassWithTag` "/Game/Blueprints/Dialogue/DialogueInator.DialogueInator_C" (`self.DownloadDialogueTag`)))
          (for _array_element _outactors
            (bind _asdialogue_inator (cast `/Game/Blueprints/Dialogue/DialogueInator` _array_element))
            (`/Game/Blueprints/Dialogue/DialogueInator.ReEnableDialogue` _asdialogue_inator)
            (`/Game/Blueprints/Dialogue/DialogueInator.UnDisplace` _asdialogue_inator)))))))

(event `LockPlayer`
  (params (CanInteract :type Boolean))
  (set `self.CanInteract` CanInteract))

(fn `UserConstructionScript`)