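; Inspectable pen object that the player picks up to examine up close and rotate, then returns to its original transform.
; Interact alternates between inspecting and releasing, toggling movement, look input, cursor and camera blur, and pausing or resuming the Chronovert timer.
; A timeline lerps the object to the character's inspect point, where mouse and IA_Move input rotate it.
; Look-target events toggle the widget's visibility.
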(event `self.ReceiveTick`
  (params (DeltaSeconds :type "Float (single-precision)"))
  (if (`self.CanInspect`) :!label _label
    (`SceneComponent.K2_AddLocalRotation` (`self.Object`) (`KismetMathLibrary.MakeRotator` (* (stale `InputAxisKey|MouseX` AxisValue) 0.4) (* (stale `InputAxisKey|MouseY` AxisValue) 0.4)) false false)))

(event `InputAxisKey|MouseX`
  (params (AxisValue :type "Float (single-precision)"))
  (goto _label))

(event `InputAxisKey|MouseY`
  (params (AxisValue :type "Float (single-precision)"))
  (goto _label))

(event `EnhancedInput|/Game/Input/Actions/IA_Move`
  (params (ActionValue :type "Vector2D Structure") (ElapsedSeconds :type "Float (double-precision)") (TriggeredSeconds :type "Float (double-precision)") (InputAction :type "InputAction Object Reference" :default "/Game/Input/Actions/IA_Move.IA_Move"))
  (:`Triggered`
    (if (`self.CanInspect`)
      (`SceneComponent.K2_AddLocalRotation` (`self.Object`) (`KismetMathLibrary.MakeRotator` (* ActionValue_X 1.0) (* ActionValue_Y 1.0)) false false))))

(event `self.ReceiveBeginPlay`
  (bind _object (`self.Object`))
  (set `self.Original Loc` (`SceneComponent.K2_GetComponentLocation` _object))
  (set `self.Original Rot` (`SceneComponent.K2_GetComponentRotation` _object))
  (`self.EnableInput` (`GameplayStatics.GetPlayerController` 0)))

(event `self.Interact`
  (params (InteractingActor :type "Actor Object Reference"))
  (bind _returnvalue (`GameplayStatics.GetPlayerController` 0))
  (bind _returnvalue_2 (`GameplayStatics.GetPlayerCharacter` 0))
  (bind _object (`self.Object`))
  (bind _widget (`self.Widget`))
  (`InteractableInterface.InteractPauseChronovertTimer`)
  (if (`self.CanInteract`)
    (`/Engine/EditorBlueprintResources/StandardMacros.FlipFlop`
      (:`A`
        (`SceneComponent.SetVisibility` _widget false false)
        (`/Engine/EditorBlueprintResources/StandardMacros.DoOnce` false :!label _label_2
          (:`Completed`
            (set `self.CanShowWidget` false)
            (set `PlayerController.bShowMouseCursor` true (`GameplayStatics.GetPlayerController` 0))
            (set `self.CanInspect` true)
            (set `self.CanInteract` false)
            (bind _asbp_first_person_character (cast `/Game/FirstPerson/Blueprints/BP_FirstPersonCharacter` (`GameplayStatics.GetPlayerCharacter` 0)))
            (bind _asbp_first_person_character_2 (cast `/Game/FirstPerson/Blueprints/BP_FirstPersonCharacter` _returnvalue_2))
            (`/Game/FirstPerson/Blueprints/BP_FirstPersonCharacter.SetInspectCamBlur` _asbp_first_person_character_2 true 0.0)
            (`CharacterMovementComponent.DisableMovement` (`Character.CharacterMovement` _returnvalue_2))
            (`Controller.SetIgnoreLookInput` (`GameplayStatics.GetPlayerController` 0) true)
            (bind (_direction _newtrack_0) (`Timeline|Timeline` :!via `PlayFromStart`)
              (:`Update`
                (bind (_returnvalue_location _returnvalue_rotation) (`KismetMathLibrary.BreakTransform` (`SceneComponent.K2_GetComponentToWorld` (`/Game/FirstPerson/Blueprints/BP_FirstPersonCharacter.IObjectPoint` _asbp_first_person_character))))
                (`SceneComponent.K2_SetWorldTransform` (`self.Object`) (`KismetMathLibrary.MakeTransform` (`KismetMathLibrary.VLerp` (`SceneComponent.K2_GetComponentLocation` _object) _returnvalue_location _newtrack_0) (`KismetMathLibrary.RLerp` (`SceneComponent.K2_GetComponentRotation` _object) _returnvalue_rotation _newtrack_0)) false false))
              (:`Finished`
                (set `self.CanInteract` true))))))
      (:`B`
        (`SceneComponent.SetVisibility` _widget true false)
        (`|ExecutionSequence`
          (:`then_0`
            (goto _label_2 :!via `Reset`))
          (:`then_1`
            (set `self.CanInspect` false)
            (set `self.CanShowWidget` true)
            (`CharacterMovementComponent.SetMovementMode` (`Character.CharacterMovement` (`GameplayStatics.GetPlayerCharacter` 0)) "MOVE_Walking" 0)
            (set `PlayerController.bShowMouseCursor` false _returnvalue)
            (`Controller.ResetIgnoreLookInput` _returnvalue)
            (`WidgetBlueprintLibrary.SetInputMode_GameOnly` _returnvalue)
            (`SceneComponent.K2_SetWorldTransform` (`self.Object`) (`KismetMathLibrary.MakeTransform` (`self.Original Loc`) (`self.Original Rot`)) false false)
            (set `self.CanInteract` true)
            (bind _asbp_first_person_character_3 (cast `/Game/FirstPerson/Blueprints/BP_FirstPersonCharacter` (`GameplayStatics.GetPlayerCharacter` 0)))
            (`/Game/FirstPerson/Blueprints/BP_FirstPersonCharacter.SetInspectCamBlur` _asbp_first_person_character_3 false 0.0)
            (`InteractableInterface.InteractResumeChronovertTimer`)))))))

(event `self.LookTargetEvent`
  (params (isLooking :type Boolean))
  (bind _widget (`self.Widget`))
  ; Enable/Disable Widget
  (`self.CanShowWidget`
    (:`then`
      (if isLooking
        (`SceneComponent.SetVisibility` _widget true false)
        (else
          (`SceneComponent.SetVisibility` _widget false false))))
    (:`else`)))

(fn `UserConstructionScript`)