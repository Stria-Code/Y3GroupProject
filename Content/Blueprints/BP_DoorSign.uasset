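; BP_DoorSign is a door sign whose text colour shows whether it is active.
; On BeginPlay the text render takes the on or off colour according to StartOn.
; SetTechActive plays or reverses the SignLights timeline, whose Activation track blends the text between the off and on colours in linear colour space.
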(event `self.ReceiveBeginPlay`
  (bind _textrender (`self.TextRender`))
  (if (`self.StartOn`)
    (`TextRenderComponent.SetTextRenderColor` _textrender (`self.OnColour`))
    (else
      (`TextRenderComponent.SetTextRenderColor` _textrender (`self.OffColour`)))))

(event `/Game/Blueprints/Interface/BPI_Tech.SetTechActive`
  (params (IsActive :type Boolean))
  (if IsActive
    (bind (_direction _activation) (`Timeline|SignLights` :!label _label)
      (:`Update`
        (`TextRenderComponent.SetTextRenderColor` (`self.TextRender`) (`KismetMathLibrary.Conv_LinearColorToColor` (`KismetMathLibrary.LinearColorLerp` (`KismetMathLibrary.Conv_ColorToLinearColor` (`self.OffColour`)) (`KismetMathLibrary.Conv_ColorToLinearColor` (`self.OnColour`)) _activation)))))
    (else
      (goto _label :!via `Reverse`))))

(fn `UserConstructionScript`)